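; Grabbable stamp for the stamping minigame, with mesh and color set by its Blue, Red or Green group.
; While held it follows the cursor with clamped height and shows a decal indicator.
; BeginStamp traces downward and plays a down-and-back timeline, succeeding only on an unstamped BP_StampArea of the matching group.
; Success spawns decal and VFX and advances the paper's stamp count; failure triggers error effects and interrupts the animation.
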(event `self.ReceiveBeginPlay`
  (bind _cube (`self.Cube`))
  (set `self.OriginalRotation` (`SceneComponent.K2_GetComponentRotation` (`self.Cube`)))
  (set `self.OriginalLocation` (`SceneComponent.K2_GetComponentLocation` (`self.Cube`)))
  (bind _returnvalue (`PrimitiveComponent.CreateDynamicMaterialInstance` _cube 1 (`PrimitiveComponent.GetMaterial` _cube 1) "None"))
  (set `self.StampDynamicMaterialInstance` _returnvalue)
  (`self.CreateDynamicEffectMaterials`)
  (`self.SetStampColor`)
  (`self.SetStampMesh`))

(event `/Game/Libraries/Minigames/BPI_MinigameInteractable.MinigameInteractedStart`
  (params (PlayerActor :type "Actor Object Reference") (CursorWorldLocation :type "Vector Structure") (CursorWorldDirection :type "Vector Structure") (CursorHitLocation :type "Vector Structure"))
  (bind _cube (`self.Cube`))
  (`PrimitiveComponent.SetSimulatePhysics` _cube false)
  (`SceneComponent.K2_SetWorldRotation` _cube (`self.OriginalRotation`) false false)
  (set `self.IsInteracting` true)
  (`MaterialInstanceDynamic.SetScalarParameterValue` (`self.IndicatorDMI`) "Opacity" 1.0)
  (`/Game/Features/Stamping/ToPlace/BP_StampMinigame.Event CursorInteracts` (`self.StampMinigameRef`)))

(event `/Game/Libraries/Minigames/BPI_MinigameInteractable.MinigameInteractedEnded`
  (params (PlayerActor :type "Actor Object Reference") (CursorWorldLocation :type "Vector Structure") (CursorWorldDirection :type "Vector Structure") (CursorHitLocation :type "Vector Structure"))
  (`PrimitiveComponent.SetSimulatePhysics` (`self.Cube`) true)
  (set `self.IsInteracting` false)
  (`MaterialInstanceDynamic.SetScalarParameterValue` (`self.IndicatorDMI`) "Opacity" 0.0)
  (`/Game/Features/Stamping/ToPlace/BP_StampMinigame.Event CursorDefault` (`self.StampMinigameRef`)))

(event `/Game/Libraries/Minigames/BPI_MinigameInteractable.MinigameInteractedContinous`
  (params (PlayerActor :type "Actor Object Reference") (CursorWorldLocation :type "Vector Structure") (CursorWorldDirection :type "Vector Structure") (CursorHitLocation :type "Vector Structure"))
  (bind (_returnvalue_x _returnvalue_y _returnvalue_z) (`KismetMathLibrary.BreakVector` (+ CursorWorldLocation CursorWorldDirection CursorHitLocation)))
  (bind (_itempickupheight_x _itempickupheight_y) (`KismetMathLibrary.BreakVector2D` (`/Game/Features/Stamping/ToPlace/BP_StampMinigame.ItemPickupHeight` (`self.StampMinigameRef`))))
  (if (`self.IsInteracting`)
    (if (not (`self.bIsStamping`))
      (`self.K2_SetActorLocation` (`KismetMathLibrary.MakeVector` _returnvalue_x _returnvalue_y (`KismetMathLibrary.FClamp` _returnvalue_z _itempickupheight_x _itempickupheight_y)))
      (bind (_start _end) (`self.GetPositionDown`)))))

(event `Event BeginStamp`
  (bind _stampminigameref (`self.StampMinigameRef`))
  (bind _stampminigameref_2 (`self.StampMinigameRef`))
  (bind _currentpaperref (`/Game/Features/Stamping/ToPlace/BP_StampMinigame.CurrentPaperRef` (`self.StampMinigameRef`)))
  (`GameplayStatics.PlaySoundAtLocation` "/Game/SoundAndMusic/SoundEffects/MiniGames/MS_Stamp.MS_Stamp" (`self.K2_GetActorLocation`) (struct) 1.0 1.0 0.0 null null null null)
  (if (`self.IsInteracting`)
    (if (not (`self.bIsStamping`))
      (set `self.InitialLocation` (`self.K2_GetActorLocation`))
      (bind (_start _end) (`self.GetPositionDown`))
      (bind _outhit (`KismetSystemLibrary.LineTraceSingle` :`Start` _start :`End` _end :`TraceChannel` "TraceTypeQuery1" :`DrawTime` 1.0))
      (bind (_bblockinghit _binitialoverlap _time _distance _location _impactpoint _normal _impactnormal _physmat _hitactor _hitcomponent) (`GameplayStatics.BreakHitResult` _outhit))
      (`self.NewFunction` _location _impactnormal (+ _impactpoint _impactnormal) _hitcomponent)
      (set `self.bIsStamping` true)
      (bind _asbp_stamp_area (cast `/Game/Features/Stamping/BP_StampArea` _hitactor)
        (:`then`
          (if (`/Game/Features/Stamping/BP_StampArea.Stamped` _asbp_stamp_area)
            (set `self.bCorrectStamp` false :!label _label)
            ; Stamp Animation
            (bind (_direction _alpha) (`Timeline|Timeline` :!via `PlayFromStart` :!label _label_2)
              (:`Update`
                (`self.MoveStampToTargetLocation` _alpha)
                ; Stamp VFX
                (if (>= _alpha 0.25)
                  (`/Engine/EditorBlueprintResources/StandardMacros.DoOnce` false :!label _label_3
                    (:`Completed`
                      (if (`self.bCorrectStamp`)
                        ; Correct Stamp
                        (`GameplayStatics.PlaySoundAtLocation` "/Game/SoundAndMusic/SoundEffects/MiniGames/MS_ActionSuccess.MS_ActionSuccess" (`self.K2_GetActorLocation`) (struct) 1.0 1.0 0.0 null null null null)
                        (`self.SpawnCorrectStampVFX`)
                        (`/Game/Features/Stamping/BP_StampArea.Event DisableStampArea` (`self.StampArea`))
                        (bind _result (`/Engine/EditorBlueprintResources/StandardMacros.IncrementInt` (`/Game/Features/Stamping/BP_StampPaper.StampAmountIndex` _currentpaperref))
                          (:`  `
                            (if (== _result (`/Game/Features/Stamping/BP_StampPaper.StampAmount` _currentpaperref))
                              (set `/Game/Features/Stamping/BP_StampPaper.MarkForFinished` true (`/Game/Features/Stamping/ToPlace/BP_StampMinigame.CurrentPaperRef` (`self.StampMinigameRef`)))
                              (`PlayerController.PlayDynamicForceFeedback` (`/Game/Features/Stamping/ToPlace/BP_StampMinigame.PlayerControllerRef` _stampminigameref) (`/Game/Features/Stamping/ToPlace/BP_StampMinigame.VibrationIntensity` _stampminigameref) (`/Game/Features/Stamping/ToPlace/BP_StampMinigame.CorrectStampVibrationDuration` _stampminigameref) true true true true))))
                        (else
                          ; Incorrect Stamp
                          (`GameplayStatics.PlaySoundAtLocation` "/Game/SoundAndMusic/SoundEffects/MiniGames/MS_ActionFail.MS_ActionFail" (`self.K2_GetActorLocation`) (struct) 1.0 1.0 0.0 null null null null)
                          (`self.SpawnIncorrectStampVFX`)
                          (`|ExecutionSequence`
                            (:`then_0`
                              (`/Game/Features/Stamping/ToPlace/BP_StampMinigameInteractor.Event Pickup` (`self.StampInteractorRef`))
                              (set `self.bIsStamping` false)
                              (goto _label_2 :!via `Stop`))
                            (:`then_1`
                              (`PlayerController.PlayDynamicForceFeedback` (`/Game/Features/Stamping/ToPlace/BP_StampMinigame.PlayerControllerRef` _stampminigameref_2) (`/Game/Features/Stamping/ToPlace/BP_StampMinigame.VibrationIntensity` _stampminigameref_2) (`/Game/Features/Stamping/ToPlace/BP_StampMinigame.IncorrectStampVibractionDuration` _stampminigameref_2) true true true true)))))))
                  (else
                    (goto _label_3 :!via `Reset`))))
              (:`Finished`
                (set `self.bIsStamping` false)))
            (else
              (set `/Game/Features/Stamping/BP_StampArea.Stamped` true _asbp_stamp_area)
              (set `self.bCorrectStamp` (`|EnumEquality` (`/Game/Features/Stamping/BP_StampArea.StampGroup` _asbp_stamp_area) (`self.StampGroup`)))
              (set `self.StampArea` _asbp_stamp_area)
              (goto _label_2 :!via `PlayFromStart`))))
        (:`CastFailed`
          (goto _label))))))

(event `/Game/Features/Stamping/BPI_Hoverable.Hovered`
  (params (Hovered :type Boolean))
  (bind _stampminigameref (`self.StampMinigameRef`))
  ; Hovered Feedback
  (if Hovered
    (`/Game/Features/Stamping/ToPlace/BP_StampMinigame.Event CursorHovers` _stampminigameref)
    (`MaterialInstanceDynamic.SetScalarParameterValue` (`self.StampOverlayDMI`) "Opacity" 1.0)
    (bind (_direction _fade) (`Timeline|GlowFade` :!label _label_4)
      (:`Update`
        (`MaterialInstanceDynamic.SetScalarParameterValue` (`self.StampDynamicMaterialInstance`) "GlowStrainght" _fade)))
    (else
      (`/Game/Features/Stamping/ToPlace/BP_StampMinigame.Event CursorDefault` _stampminigameref)
      (`MaterialInstanceDynamic.SetScalarParameterValue` (`self.StampOverlayDMI`) "Opacity" 0.0)
      (goto _label_4 :!via `Reverse`))))

(fn `CreateDynamicEffectMaterials`
  (bind _returnvalue (`DecalComponent.CreateDynamicMaterialInstance` (`self.DecalIndicator`)))
  (bind _output_get (set `self.IndicatorDMI` _returnvalue))
  (`MaterialInstanceDynamic.SetScalarParameterValue` _output_get "EmissiveColor LUT" (`self.StampColor`))
  (`MaterialInstanceDynamic.SetScalarParameterValue` (`self.IndicatorDMI`) "Opacity" 0.0)
  (bind _returnvalue_2 (`KismetMaterialLibrary.CreateDynamicMaterialInstance` "/Game/Vfx/Stamping/M_VFX_StampDecal.M_VFX_StampDecal"))
  (set `self.DecalDMI` _returnvalue_2)
  (bind _returnvalue_3 (`KismetMaterialLibrary.CreateDynamicMaterialInstance` "/Game/Vfx/Materials/M_VFX_Hovered.M_VFX_Hovered"))
  (bind _output_get_2 (set `self.StampOverlayDMI` _returnvalue_3))
  (`MeshComponent.SetOverlayMaterial` (`self.Cube`) _output_get_2))

(fn `GetPositionDown`
  (returns (Start :type "Vector Structure") (End :type "Vector Structure"))
  (bind _returnvalue (`SceneComponent.K2_GetComponentLocation` (`self.Cube`)))
  (return _returnvalue (+ _returnvalue (* (`KismetMathLibrary.Vector_Down`) 100.0))))

(fn `IsHovered`
  (params (in :type Boolean))
  (returns (out :type Boolean))
  (bind _output_get (set `self.bIsHovered` in))
  (return _output_get))

(fn `MoveStampToTargetLocation`
  (params (Alpha :type "Float (double-precision)"))
  (if (<= Alpha 0.5)
    (`self.K2_SetActorLocation` (`KismetMathLibrary.VLerp` (`self.InitialLocation`) (`self.TargetLocation`) Alpha))
    (else
      (`self.K2_SetActorLocation` (`KismetMathLibrary.VLerp` (`self.TargetLocation`) (`self.InitialLocation`) Alpha)))))

(fn `NewFunction`
  (params (ImpactLocation :type "Vector Structure") (ImpactNormal :type "Vector Structure") (TargetLocation :type "Vector Structure") (`Hit Component` :type "PrimitiveComponent Object Reference"))
  (set `self.ImpactLocation` ImpactLocation)
  (set `self.ImpactNormal` ImpactNormal)
  (set `self.TargetLocation` TargetLocation)
  (set `self.Hit Component` `Hit Component`))

(fn `SetStampColor`
  (switch `/Game/Libraries/Minigames/E_StampGroup` (`self.StampGroup`)
    (:`NewEnumerator0`
      (bind _output_get (set `self.StampColor` 1.0))
      ; StampMesh
      (`MaterialInstanceDynamic.SetScalarParameterValue` (`self.StampDynamicMaterialInstance`) "TintColor LUT" _output_get)
      (`MaterialInstanceDynamic.SetScalarParameterValue` (`self.StampDynamicMaterialInstance`) "EmissiveColor LUT" _output_get)
      (`MaterialInstanceDynamic.SetScalarParameterValue` (`self.IndicatorDMI`) "EmissiveColor LUT" _output_get)
      (`MaterialInstanceDynamic.SetScalarParameterValue` (`self.StampOverlayDMI`) "EmissiveColor LUT" _output_get)
      (`MaterialInstanceDynamic.SetScalarParameterValue` (`self.StampOverlayDMI`) "Opacity" 0.0)
      ; Decals
      (`MaterialInstanceDynamic.SetScalarParameterValue` (`self.DecalDMI`) "EmissiveColor LUT" _output_get)
      (`MaterialInstanceDynamic.SetVectorParameterValue` (`self.DecalDMI`) "ChannelToPick" (struct :`R` 1.0 :`A` 1.0))
      (`MaterialInstanceDynamic.SetVectorParameterValue` (`self.IndicatorDMI`) "ChannelToPick" (struct :`R` 1.0 :`A` 1.0)))
    (:`NewEnumerator1`
      (bind _output_get_2 (set `self.StampColor` 5.0))
      (`MaterialInstanceDynamic.SetScalarParameterValue` (`self.StampDynamicMaterialInstance`) "TintColor LUT" _output_get_2)
      (`MaterialInstanceDynamic.SetScalarParameterValue` (`self.StampDynamicMaterialInstance`) "EmissiveColor LUT" _output_get_2)
      (`MaterialInstanceDynamic.SetScalarParameterValue` (`self.IndicatorDMI`) "EmissiveColor LUT" _output_get_2)
      (`MaterialInstanceDynamic.SetScalarParameterValue` (`self.StampOverlayDMI`) "EmissiveColor LUT" _output_get_2)
      (`MaterialInstanceDynamic.SetScalarParameterValue` (`self.StampOverlayDMI`) "Opacity" 0.0)
      (`MaterialInstanceDynamic.SetScalarParameterValue` (`self.DecalDMI`) "EmissiveColor LUT" _output_get_2)
      (`MaterialInstanceDynamic.SetVectorParameterValue` (`self.DecalDMI`) "ChannelToPick" (struct :`B` 1.0 :`A` 1.0))
      (`MaterialInstanceDynamic.SetVectorParameterValue` (`self.IndicatorDMI`) "ChannelToPick" (struct :`B` 1.0 :`A` 1.0)))
    (:`NewEnumerator2`
      (bind _output_get_3 (set `self.StampColor` 3.0))
      (`MaterialInstanceDynamic.SetScalarParameterValue` (`self.StampDynamicMaterialInstance`) "TintColor LUT" _output_get_3)
      (`MaterialInstanceDynamic.SetScalarParameterValue` (`self.StampDynamicMaterialInstance`) "EmissiveColor LUT" _output_get_3)
      (`MaterialInstanceDynamic.SetScalarParameterValue` (`self.IndicatorDMI`) "EmissiveColor LUT" _output_get_3)
      (`MaterialInstanceDynamic.SetScalarParameterValue` (`self.StampOverlayDMI`) "EmissiveColor LUT" _output_get_3)
      (`MaterialInstanceDynamic.SetScalarParameterValue` (`self.StampOverlayDMI`) "Opacity" 0.0)
      (`MaterialInstanceDynamic.SetScalarParameterValue` (`self.DecalDMI`) "EmissiveColor LUT" _output_get_3)
      (`MaterialInstanceDynamic.SetVectorParameterValue` (`self.DecalDMI`) "ChannelToPick" (struct :`G` 1.0 :`A` 1.0))
      (`MaterialInstanceDynamic.SetVectorParameterValue` (`self.IndicatorDMI`) "ChannelToPick" (struct :`G` 1.0 :`A` 1.0))))
  (`MaterialInstanceDynamic.SetScalarParameterValue` (`self.StampDynamicMaterialInstance`) "GlowStrainght" 3.0))

(fn `SetStampMesh`
  (bind _cube (`self.Cube`))
  (switch `/Game/Libraries/Minigames/E_StampGroup` (`self.StampGroup`)
    (:`NewEnumerator0`
      (`StaticMeshComponent.SetStaticMesh` _cube "/Game/Environment/Assets/Stamp/ME_Envi_Stamp2.ME_Envi_Stamp2"))
    (:`NewEnumerator1`
      (`StaticMeshComponent.SetStaticMesh` _cube "/Game/Environment/Assets/Stamp/ME_Envi_Stamp1.ME_Envi_Stamp1"))
    (:`NewEnumerator2`
      (`StaticMeshComponent.SetStaticMesh` _cube "/Game/Environment/Assets/Stamp/ME_Envi_Stamp3.ME_Envi_Stamp3"))))

(fn `SpawnCorrectStampVFX`
  (bind _returnvalue (`NiagaraFunctionLibrary.SpawnSystemAtLocation` "/Game/Vfx/ParticleSystems/FXS_VFX_Stamp_Correct_01.FXS_VFX_Stamp_Correct_01" (`self.TargetLocation`) (struct) (1.0 1.0 1.0) true false "AutoRelease"))
  (`NiagaraComponent.SetVariableFloat` _returnvalue "User.SetColor" (`self.StampColor`))
  (`ActorComponent.Activate` _returnvalue false)
  (bind _returnvalue_2 (`GameplayStatics.SpawnDecalAttached` (`self.DecalDMI`) (3.0 3.0 3.0) (`self.Hit Component`) "None" (`self.ImpactLocation`) (`KismetMathLibrary.Conv_VectorToRotator` (`self.ImpactNormal`)) "KeepWorldPosition"))
  (`KismetArrayLibrary.Array_Add` (`self.SpawnedDecals`) _returnvalue_2)
  (`MaterialInstanceDynamic.SetScalarParameterValue` (`self.DecalDMI`) "EmissiveColor LUT" (`self.StampColor`))
  (`MaterialInstanceDynamic.SetScalarParameterValue` (`self.DecalDMI`) "Glow Strength" 8.0))

(fn `SpawnIncorrectStampVFX`
  (`ActorComponent.Activate` (`self.ElectricEffect`) true)
  (`ActorComponent.Activate` (`self.FXS_VFX_InkImpact_Stample_01`) false)
  (`self.OnStampIncorrect` (`self.StampInteractorRef`)))

(fn `UserConstructionScript`)