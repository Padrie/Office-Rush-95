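; A draggable paper in the paper-sorting minigame, randomly assigned to a blue, red or green group at BeginPlay.
; Its group sets LUT parameters on a dynamic material, while SelectPaperTexture can swap in one of five texture sets.
; While held, physics is off and it follows the cursor within a clamped height.
; A downward multi-trace sends hover messages to actors beneath, and interaction events update the minigame's cursor.
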(event `self.ReceiveBeginPlay`
  (bind _paper (`self.Paper`))
  (set `self.OriginalLocation` (`SceneComponent.K2_GetComponentLocation` (`self.Paper`)))
  (bind _returnvalue (`PrimitiveComponent.CreateDynamicMaterialInstance` _paper 0 (`PrimitiveComponent.GetMaterial` _paper 0) "None"))
  (set `self.StampDynamicMaterialInstance` _returnvalue)
  (`self.SetRandomColor`)
  (`PrimitiveComponent.SetSimulatePhysics` (`self.Paper`) false))

(event `/Game/Libraries/Minigames/BPI_MinigameInteractable.MinigameInteractedStart`
  (params (PlayerActor :type "Actor Object Reference") (CursorWorldLocation :type "Vector Structure") (CursorWorldDirection :type "Vector Structure") (CursorHitLocation :type "Vector Structure"))
  (bind _paper (`self.Paper`))
  (if (not (`self.IsFinished`))
    (`PrimitiveComponent.SetSimulatePhysics` _paper false)
    (`SceneComponent.K2_SetWorldRotation` _paper (`self.OriginalRotation`) false false)
    (set `self.IsInteracting` true)))

(event `/Game/Libraries/Minigames/BPI_MinigameInteractable.MinigameInteractedEnded`
  (params (PlayerActor :type "Actor Object Reference") (CursorWorldLocation :type "Vector Structure") (CursorWorldDirection :type "Vector Structure") (CursorHitLocation :type "Vector Structure"))
  (if (not (`self.IsFinished`))
    (`PrimitiveComponent.SetSimulatePhysics` (`self.Paper`) true)
    (set `self.IsInteracting` false)
    (`/Game/Features/PaperSorting/BP_SortingMinigame.Event CursorDefault` (`self.SortMinigameRef`))))

(event `/Game/Libraries/Minigames/BPI_MinigameInteractable.MinigameInteractedContinous`
  (params (PlayerActor :type "Actor Object Reference") (CursorWorldLocation :type "Vector Structure") (CursorWorldDirection :type "Vector Structure") (CursorHitLocation :type "Vector Structure"))
  (bind (_returnvalue_x _returnvalue_y _returnvalue_z) (`KismetMathLibrary.BreakVector` (+ CursorWorldLocation CursorWorldDirection CursorHitLocation)))
  (bind _lasthoveredactor (`self.LastHoveredActor`))
  (bind (_paperpickupheight_x _paperpickupheight_y) (`KismetMathLibrary.BreakVector2D` (`/Game/Features/PaperSorting/BP_SortingMinigame.PaperPickupHeight` (`self.SortMinigameRef`))))
  (bind _returnvalue (`KismetMathLibrary.MakeVector` _returnvalue_x _returnvalue_y (`KismetMathLibrary.FClamp` _returnvalue_z _paperpickupheight_x _paperpickupheight_y)))
  (if (`self.IsFinished`)
    _
    (elif (`self.IsInteracting`)
      (`SceneComponent.K2_SetWorldLocation` (`self.Paper`) _returnvalue false false)
      (bind _outhits (`KismetSystemLibrary.LineTraceMulti` _returnvalue (+ _returnvalue (0.0 0.0 -100.0)) "TraceTypeQuery1"))
      (for _array_element _outhits
        (bind (_bblockinghit _binitialoverlap _time _distance _location _impactpoint _normal _impactnormal _physmat _hitactor) (`GameplayStatics.BreakHitResult` _array_element))
        (if (!= _hitactor _lasthoveredactor)
          (`|ExecutionSequence`
            (:`then_0`
              (`/Engine/EditorBlueprintResources/StandardMacros.IsValid` _lasthoveredactor
                (:`Is Valid`
                  (message `/Game/Features/Stamping/BPI_Hoverable.Hovered` _lasthoveredactor false))))
            (:`then_1`
              (`/Engine/EditorBlueprintResources/StandardMacros.IsValid` _hitactor
                (:`Is Valid`
                  (message `/Game/Features/Stamping/BPI_Hoverable.Hovered` _hitactor true))))
            (:`then_2`
              (set `self.LastHoveredActor` _hitactor))
            (:`then_3`
              (`/Game/Features/PaperSorting/BP_SortingMinigame.Event CursorInteracts` (`self.SortMinigameRef`)))))))))

(event `/Game/Features/Stamping/BPI_Hoverable.Hovered`
  (params (Hovered :type Boolean))
  (bind _sortminigameref (`self.SortMinigameRef`))
  (if Hovered
    (if (not (`/Game/Features/PaperSorting/BP_SortingMinigameInteractor.IsInteracting` (`self.SortInteractorRef`)))
      (`/Game/Features/PaperSorting/BP_SortingMinigame.Event CursorHovers` _sortminigameref))
    (else
      (`/Game/Features/PaperSorting/BP_SortingMinigame.Event CursorDefault` _sortminigameref))))

(fn `SelectPaperTexture`
  (params (Index :type Integer))
  (`KismetSystemLibrary.PrintString` (`KismetStringLibrary.Conv_IntToString` Index))
  (switch `int` Index
    (:`0`
      (bind _returnvalue (`PrimitiveComponent.CreateDynamicMaterialInstance` (`self.Paper`) 0 "/Game/Environment/Assets/Paper/M_Inst_Papers.M_Inst_Papers" "None"))
      (`MaterialInstanceDynamic.SetTextureParameterValue` _returnvalue "Diffuse" "/Game/Environment/Assets/Paper/1/T_Envi_Paper1_BaseColor_V03.T_Envi_Paper1_BaseColor_V03")
      (`MaterialInstanceDynamic.SetTextureParameterValue` _returnvalue "Emissive Mask" "/Game/Environment/Assets/Paper/1/T_Envi_Paper1_Emissive_V03.T_Envi_Paper1_Emissive_V03"))
    (:`1`
      (bind _returnvalue_2 (`PrimitiveComponent.CreateDynamicMaterialInstance` (`self.Paper`) 0 "/Game/Environment/Assets/Paper/M_Inst_Papers.M_Inst_Papers" "None"))
      (`MaterialInstanceDynamic.SetTextureParameterValue` _returnvalue_2 "Diffuse" "/Game/Environment/Assets/Paper/2/T_Envi_Paper2_BaseColor_V03.T_Envi_Paper2_BaseColor_V03")
      (`MaterialInstanceDynamic.SetTextureParameterValue` _returnvalue_2 "Emissive Mask" "/Game/Environment/Assets/Paper/2/T_Envi_Paper2_Emissive_V03.T_Envi_Paper2_Emissive_V03"))
    (:`2`
      (bind _returnvalue_3 (`PrimitiveComponent.CreateDynamicMaterialInstance` (`self.Paper`) 0 "/Game/Environment/Assets/Paper/M_Inst_Papers.M_Inst_Papers" "None"))
      (`MaterialInstanceDynamic.SetTextureParameterValue` _returnvalue_3 "Diffuse" "/Game/Environment/Assets/Paper/3/T_Envi_Paper3_BaseColor_V03.T_Envi_Paper3_BaseColor_V03")
      (`MaterialInstanceDynamic.SetTextureParameterValue` _returnvalue_3 "Emissive Mask" "/Game/Environment/Assets/Paper/3/T_Envi_Paper3_Emissive_V03.T_Envi_Paper3_Emissive_V03"))
    (:`3`
      (bind _returnvalue_4 (`PrimitiveComponent.CreateDynamicMaterialInstance` (`self.Paper`) 0 "/Game/Environment/Assets/Paper/M_Inst_Papers.M_Inst_Papers" "None"))
      (`MaterialInstanceDynamic.SetTextureParameterValue` _returnvalue_4 "Diffuse" "/Game/Environment/Assets/Paper/4/T_Envi_Paper4_BaseColor_V03.T_Envi_Paper4_BaseColor_V03")
      (`MaterialInstanceDynamic.SetTextureParameterValue` _returnvalue_4 "Emissive Mask" "/Game/Environment/Assets/Paper/4/T_Envi_Paper4_Emissive_V03.T_Envi_Paper4_Emissive_V03"))
    (:`4`
      (bind _returnvalue_5 (`PrimitiveComponent.CreateDynamicMaterialInstance` (`self.Paper`) 0 "/Game/Environment/Assets/Paper/M_Inst_Papers.M_Inst_Papers" "None"))
      (`MaterialInstanceDynamic.SetTextureParameterValue` _returnvalue_5 "Diffuse" "/Game/Environment/Assets/Paper/5/T_Envi_Paper5_BaseColor_V03.T_Envi_Paper5_BaseColor_V03")
      (`MaterialInstanceDynamic.SetTextureParameterValue` _returnvalue_5 "Emissive Mask" "/Game/Environment/Assets/Paper/5/T_Envi_Paper5_Emissive_V03.T_Envi_Paper5_Emissive_V03"))))

(fn `SetRandomColor`
  (returns (SortingGroup :type "/Game/Features/PaperSorting/E_PaperSortingGroups Enum"))
  (bind _stampdynamicmaterialinstance (`self.StampDynamicMaterialInstance`))
  (bind _stampdynamicmaterialinstance_2 (`self.StampDynamicMaterialInstance`))
  (bind _stampdynamicmaterialinstance_3 (`self.StampDynamicMaterialInstance`))
  (bind _output_get (set `self.PaperSortingGroup` (cast `/Game/Features/PaperSorting/E_PaperSortingGroups` (`KismetMathLibrary.Conv_IntToByte` (`KismetMathLibrary.RandomInteger` 3)))))
  (`|ExecutionSequence`
    (:`then_0`
      (switch `/Game/Features/PaperSorting/E_PaperSortingGroups` _output_get
        (:`NewEnumerator0`
          (bind _output_get_2 (set `self.PaperColor` 1.0))
          (`MaterialInstanceDynamic.SetScalarParameterValue` _stampdynamicmaterialinstance "TintColor LUT" _output_get_2)
          (`MaterialInstanceDynamic.SetScalarParameterValue` _stampdynamicmaterialinstance "EmissiveColor LUT" _output_get_2))
        (:`NewEnumerator1`
          (bind _output_get_3 (set `self.PaperColor` 5.0))
          (`MaterialInstanceDynamic.SetScalarParameterValue` _stampdynamicmaterialinstance_2 "TintColor LUT" _output_get_3)
          (`MaterialInstanceDynamic.SetScalarParameterValue` _stampdynamicmaterialinstance_2 "EmissiveColor LUT" _output_get_3))
        (:`NewEnumerator2`
          (bind _output_get_4 (set `self.PaperColor` 3.0))
          (`MaterialInstanceDynamic.SetScalarParameterValue` _stampdynamicmaterialinstance_3 "TintColor LUT" _output_get_4)
          (`MaterialInstanceDynamic.SetScalarParameterValue` _stampdynamicmaterialinstance_3 "EmissiveColor LUT" _output_get_4))))
    (:`then_1`
      (return _output_get))))

(fn `UserConstructionScript`)