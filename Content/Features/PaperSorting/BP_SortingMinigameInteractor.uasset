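; Pawn that a player possesses at the paper-sorting desk to play the stamping minigame, after an authorization-token check.
; It caches the previous pawn, swaps to the task input context, and on exit restores both and restarts the minigame.
; Clamped look aims a sphere trace for hovering, picking up items and stamping.
; Tick also returns fallen papers to spawn, and a wrong stamp drives a timeline post-process glitch.
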(event `self.ReceiveBeginPlay`
  (set `self.InitialCameraRotation` (`SceneComponent.K2_GetComponentRotation` (`self.Camera`)))
  ; Post Process Setup
  (set `self.CameraOriginalRotation` (`SceneComponent.K2_GetComponentRotation` (`self.Camera`)))
  (for _array_element _
    (add `/Game/Features/Stamping/ToPlace/BP_Stamp.OnStampIncorrect` _array_element (delegate `HandleStampIncorrect`)))
  (bind _returnvalue (`KismetMaterialLibrary.CreateDynamicMaterialInstance` "/Game/Vfx/Materials/M_VFX_PP_Shocked.M_VFX_PP_Shocked"))
  (bind _output_get (set `self.Dynamic Glitch Material` _returnvalue))
  (set `CameraComponent.PostProcessSettings` (make `PostProcessSettings` :`WeightedBlendables` (make `WeightedBlendables` (`|MakeArray` (make `WeightedBlendable` 1.0 _output_get)))) (`self.Camera`)))

(event `HandleStampIncorrect`
  (params (FailedPlayer :type "/Game/Features/Stamping/ToPlace/BP_StampMinigameInteractor Object Reference"))
  ; Post Process Intensity
  (if (== FailedPlayer self)
    (bind (_direction _blend_weight) (`Timeline|Timeline` :!via `PlayFromStart`)
      (:`Update`
        (`MaterialInstanceDynamic.SetScalarParameterValue` (`self.Dynamic Glitch Material`) "Intensity" _blend_weight)))))

(event `EnhancedInput|/Game/UX/IA_Canceling`
  (params (ActionValue :type Boolean) (ElapsedSeconds :type "Float (double-precision)") (TriggeredSeconds :type "Float (double-precision)") (InputAction :type "InputAction Object Reference" :default "/Game/UX/IA_Canceling.IA_Canceling"))
  ; Exit Minigame
  (:`Triggered`
    (`self.ExitMinigame`)))

(event `Event Possess Interactor`
  (params (Interactor :type "Actor Object Reference"))
  (bind _sortingminigameref (`self.SortingMinigameRef`))
  (bind (_authorizedtokens_datatable _authorizedtokens_rowname) (break `DataTableRowHandle` (`/Game/Features/PaperSorting/BP_SortingMinigame.AuthorizedTokens` (`self.SortingMinigameRef`))))
  (bind _returnvalue (pcsubsystem `EnhancedInputLocalPlayerSubsystem` (`/Game/Features/PaperSorting/BP_SortingMinigame.PlayerControllerRef` (`self.SortingMinigameRef`))))
  ; Take control of this pawn if authorized
  (bind _asbpi_authorizer (cast `/Game/Libraries/Authorization/BPI_Authorizer` Interactor))
  (bind _returnvalue_2 (`|GetDataTableRow` "/Game/Libraries/Authorization/DT_AuthorizationTokens.DT_AuthorizationTokens" _authorizedtokens_rowname)
    (:`then`
      (bind _isauthorized (`/Game/Libraries/Authorization/BPI_Authorizer.CheckAuthorization` _asbpi_authorizer (`|MakeArray` _returnvalue_2)))
      (if _isauthorized
        (`|ExecutionSequence`
          (:`then_0`
            ; Cache the previous Pawn
            (bind _aspawn (cast `Pawn` Interactor))
            (bind _asbpi_cache (cast `/Game/Libraries/Cache/BPI_Cache` (`self.GetController` _aspawn)))
            (`/Game/Libraries/Cache/BPI_Cache.Cache` _asbpi_cache Interactor))
          (:`then_1`
            (bind _asbpi_controller (cast `/Game/Libraries/Controlling/BPI_Controller` Interactor))
            (`/Game/Libraries/Controlling/BPI_Controller.TakeControl` _asbpi_controller self)
            (`EnhancedInputSubsystemInterface.AddMappingContext` _returnvalue "/Game/Input/IMC_Tasks.IMC_Tasks" 0 (struct))
            (`EnhancedInputSubsystemInterface.RemoveMappingContext` _returnvalue "/Game/Input/IMC_Default.IMC_Default" (struct))
            (`self.SetPlayerPosition`)
            (set `/Game/Features/PaperSorting/BP_SortingDesk.Interacted` true (`/Game/Features/PaperSorting/BP_SortingMinigame.SortingDesk` (`self.SortingMinigameRef`)))
            (`/Game/Players/BP_PlayerController.OnMinigameEnteredOnce` (`/Game/Features/PaperSorting/BP_SortingMinigame.PlayerControllerRef` (`self.SortingMinigameRef`)) 1)
            (`/Game/Players/BP_PlayerCharacter.Event MinigameEntered` (`/Game/Features/PaperSorting/BP_SortingMinigame.PlayerCharacterRef` (`self.SortingMinigameRef`)))))
        (else
          (`|ExecutionSequence`
            (:`then_0`
              (`GameplayStatics.PlaySoundAtLocation` "/Game/SoundAndMusic/SoundEffects/InteractionSounds/MS_InteractionFail.MS_InteractionFail" (`self.K2_GetActorLocation`) (struct) 1.0 1.0 0.0 null null null null)
              (`PlayerController.PlayDynamicForceFeedback` (`/Game/Features/PaperSorting/BP_SortingMinigame.PlayerControllerRef` _sortingminigameref) (`/Game/Features/PaperSorting/BP_SortingMinigame.VibrationIntensity` _sortingminigameref) (`/Game/Features/PaperSorting/BP_SortingMinigame.NoAuthorizationVibrationDuration` _sortingminigameref) true true true true))))))))

(event `EnhancedInput|/Game/Input/Actions/IA_Look`
  (params (ActionValue :type "Vector2D Structure") (ElapsedSeconds :type "Float (double-precision)") (TriggeredSeconds :type "Float (double-precision)") (InputAction :type "InputAction Object Reference" :default "/Game/Input/Actions/IA_Look.IA_Look"))
  (bind _returnvalue (`GameplayStatics.GetWorldDeltaSeconds`))
  (bind (_initialcamerarotation_roll _initialcamerarotation_pitch _initialcamerarotation_yaw) (`KismetMathLibrary.BreakRotator` (`self.InitialCameraRotation`)))
  (bind (_relativerotation_roll _relativerotation_pitch _relativerotation_yaw) (`KismetMathLibrary.BreakRotator` (`SceneComponent.RelativeRotation` (`self.Camera`))))
  (:`Triggered`
    ; Move Camera
    (bind _output (`self.ClampCameraYaw` (+ (* (* ActionValue_X _returnvalue) (`self.CameraLookSpeed`)) _relativerotation_yaw) _initialcamerarotation_yaw (`self.CameraHorizontalRange`)))
    (bind _output_2 (`self.ClampCameraPitch` (+ (* (* ActionValue_Y _returnvalue) -1.0 (`self.CameraLookSpeed`)) _relativerotation_pitch) _initialcamerarotation_pitch (`self.CameraVerticalRange`)))
    (`SceneComponent.K2_SetRelativeRotation` (`self.Camera`) (`KismetMathLibrary.MakeRotator` 0.0 _output_2 _output) false false)
    (if (`self.IsInteracting`)
      _)))

(event `self.ReceiveTick`
  (params (DeltaSeconds :type "Float (single-precision)"))
  (bind _camera (`self.Camera`))
  (bind _camera_2 (`self.Camera`))
  (bind _lasthoveredactor (`self.LastHoveredActor`))
  (bind _returnvalue (`SceneComponent.K2_GetComponentLocation` _camera_2))
  (bind (_returnvalue_x _returnvalue_y _returnvalue_z) (`KismetMathLibrary.BreakVector` (`SceneComponent.K2_GetComponentLocation` (`/Game/Features/PaperSorting/BP_SortingDesk.ItemResetHeight` (`/Game/Features/PaperSorting/BP_SortingMinigame.SortingDesk` (`self.SortingMinigameRef`))))))
  ; Item Pickup
  (`|ExecutionSequence`
    (:`then_0`
      (for _array_element (`/Game/Features/PaperSorting/BP_SortingMinigame.SpawnedPaper` (`self.SortingMinigameRef`))
        (bind _paper (`/Game/Features/PaperSorting/BP_SortingPaper.Paper` _array_element))
        (bind (_returnvalue_x_2 _returnvalue_y_2 _returnvalue_z_2) (`KismetMathLibrary.BreakVector` (`SceneComponent.K2_GetComponentLocation` _paper)))
        (if (<= _returnvalue_z_2 _returnvalue_z)
          (bind _out (`/Game/Features/PaperSorting/BP_SortingMinigame.GetPaperSpawnLocation` (`self.SortingMinigameRef`)))
          (`SceneComponent.K2_SetWorldTransform` _paper (`KismetMathLibrary.MakeTransform` (+ (.location _out) (0.0 0.0 20.0)) (.rotation _out) (`SceneComponent.K2_GetComponentScale` _paper)) false false)
          (`PrimitiveComponent.SetPhysicsLinearVelocity` _paper (0.0 0.0 0.0) false "None"))))
    (:`then_1`
      (if (stale `Event Pickup` _output_get_2)
        (message `/Game/Libraries/Minigames/BPI_MinigameInteractable.MinigameInteractedContinous` (`self.SelectedObject`) null (`SceneComponent.K2_GetComponentLocation` _camera) (`KismetMathLibrary.Conv_RotatorToVector` (`SceneComponent.K2_GetComponentRotation` _camera)) (* (`SceneComponent.GetForwardVector` _camera) (`self.HoldDistanceFromCamera`)))))
    (:`then_2`
      (bind _outhit (`KismetSystemLibrary.SphereTraceSingle` :`Start` _returnvalue :`End` (+ _returnvalue (`SceneComponent.K2_GetComponentRotation` _camera_2) (* (`SceneComponent.GetForwardVector` _camera_2) 1000)) :`Radius` 0.5 :`TraceChannel` "TraceTypeQuery1" :`DrawTime` 0.1))
      (bind (_bblockinghit _binitialoverlap _time _distance _location _impactpoint _normal _impactnormal _physmat _hitactor) (`GameplayStatics.BreakHitResult` _outhit))
      (if (!= _hitactor _lasthoveredactor)
        (`|ExecutionSequence`
          (:`then_0`
            (`/Engine/EditorBlueprintResources/StandardMacros.IsValid` _lasthoveredactor
              (:`Is Valid`
                (message `/Game/Features/Stamping/BPI_Hoverable.Hovered` _lasthoveredactor false))))
          (:`then_1`
            (`/Engine/EditorBlueprintResources/StandardMacros.IsValid` _hitactor
              (:`Is Valid`
                (message `/Game/Features/Stamping/BPI_Hoverable.Hovered` _hitactor true))))
          (:`then_2`
            (set `self.LastHoveredActor` _hitactor)))))))

(event `Event Pickup`
  (bind _camera (`self.Camera`))
  (bind _returnvalue (`SceneComponent.K2_GetComponentLocation` _camera))
  ; Item Pickup
  (if (`self.IsInteracting`) :!label _label
    (message `/Game/Libraries/Minigames/BPI_MinigameInteractable.MinigameInteractedEnded` (`self.SelectedObject`) null (0.0 0.0 0.0) (0.0 0.0 0.0) (0.0 0.0 0.0))
    (set `self.SelectedObject` null)
    (set `self.IsInteracting` false)
    (else
      (bind _outhit (`KismetSystemLibrary.SphereTraceSingle` :`Start` _returnvalue :`End` (+ _returnvalue (`SceneComponent.K2_GetComponentRotation` _camera) (* (`SceneComponent.GetForwardVector` _camera) 1000)) :`Radius` 0.5 :`TraceChannel` "TraceTypeQuery1" :`DrawTime` 1.0))
      (bind (_bblockinghit _binitialoverlap _time _distance _location _impactpoint _normal _impactnormal _physmat _hitactor) (`GameplayStatics.BreakHitResult` _outhit))
      (bind _asbp_stamp_minigame_reset_button (cast `/Game/Features/Stamping/ToPlace/BP_StampMinigameResetButton` _hitactor)
        (:`then`
          (message `/Game/Libraries/Minigames/BPI_MinigameInteractable.MinigameInteractedStart` _asbp_stamp_minigame_reset_button null (0.0 0.0 0.0) (0.0 0.0 0.0) (0.0 0.0 0.0)))
        (:`CastFailed`
          (bind _asbp_sorting_paper (cast `/Game/Features/PaperSorting/BP_SortingPaper` _hitactor)
            (:`then`
              (if (not (== (`/Game/Features/PaperSorting/BP_SortingPaper.IsFinished` _asbp_sorting_paper) true))
                (if (`KismetSystemLibrary.DoesImplementInterface` _hitactor "/Game/Libraries/Minigames/BPI_MinigameInteractable.BPI_MinigameInteractable_C") :!label _label_2
                  (bind _output_get (set `self.SelectedObject` _hitactor))
                  (message `/Game/Libraries/Minigames/BPI_MinigameInteractable.MinigameInteractedStart` _output_get null (0.0 0.0 0.0) (0.0 0.0 0.0) (0.0 0.0 0.0))
                  (bind _output_get_2 (set `self.IsInteracting` true)))))
            (:`CastFailed`
              (goto _label_2))))))))

(event `EnhancedInput|/Game/Input/Actions/IA_Pickup`
  (params (ActionValue :type Boolean) (ElapsedSeconds :type "Float (double-precision)") (TriggeredSeconds :type "Float (double-precision)") (InputAction :type "InputAction Object Reference" :default "/Game/Input/Actions/IA_Pickup.IA_Pickup"))
  ; Item Pickup
  (:`Started`
    (goto _label)))

(event `EnhancedInput|/Game/Input/Actions/IA_Interact`
  (params (ActionValue :type Boolean) (ElapsedSeconds :type "Float (double-precision)") (TriggeredSeconds :type "Float (double-precision)") (InputAction :type "InputAction Object Reference" :default "/Game/Input/Actions/IA_Interact.IA_Interact"))
  ; Stamp Action
  (:`Started`
    (if (`self.IsInteracting`)
      (bind _asbp_stamp (cast `/Game/Features/Stamping/ToPlace/BP_Stamp` (`self.SelectedObject`)))
      (`/Game/Features/Stamping/ToPlace/BP_Stamp.Event BeginStamp` _asbp_stamp))))

(fn `ClampCameraPitch`
  (params (Value :type "Float (double-precision)") (Axis :type "Float (double-precision)") (RangeValue :type "Vector2D Structure"))
  (returns (output :type "Float (double-precision)"))
  (return (`KismetMathLibrary.FClamp` Value (- Axis RangeValue_X) (+ Axis RangeValue_Y))))

(fn `ClampCameraYaw`
  (params (Value :type "Float (double-precision)") (Axis :type "Float (double-precision)") (RangeValue :type "Vector2D Structure"))
  (returns (output :type "Float (double-precision)"))
  (bind (_returnvalue_roll _returnvalue_pitch _returnvalue_yaw) (`KismetMathLibrary.BreakRotator` (`KismetMathLibrary.NormalizedDeltaRotator` (`KismetMathLibrary.MakeRotator` 0.0 0.0 Value) (`KismetMathLibrary.MakeRotator` 0.0 0.0 Axis))))
  (return (+ (`KismetMathLibrary.FClamp` _returnvalue_yaw (* RangeValue_X -1.0) RangeValue_Y) Axis)))

(fn `ExitMinigame`
  (bind _returnvalue (`self.GetController`))
  (bind _sortingminigameref (`self.SortingMinigameRef`))
  (bind _playercontrollerref (`/Game/Features/PaperSorting/BP_SortingMinigame.PlayerControllerRef` (`self.SortingMinigameRef`)))
  (bind _returnvalue_2 (pcsubsystem `EnhancedInputLocalPlayerSubsystem` (`/Game/Features/PaperSorting/BP_SortingMinigame.PlayerControllerRef` (`self.SortingMinigameRef`))))
  (message `/Game/Libraries/Minigames/BPI_MinigameInteractable.MinigameInteractedEnded` (`self.SelectedObject`) null (0.0 0.0 0.0) (0.0 0.0 0.0) (0.0 0.0 0.0))
  (set `self.SelectedObject` null)
  (set `self.IsInteracting` false)
  (bind _asbpi_cache (cast `/Game/Libraries/Cache/BPI_Cache` _returnvalue))
  (bind _actor (`/Game/Libraries/Cache/BPI_Cache.Retrieve` _asbpi_cache))
  (bind _aspawn (cast `Pawn` _actor))
  (`Controller.Possess` _returnvalue _aspawn)
  (`EnhancedInputSubsystemInterface.AddMappingContext` _returnvalue_2 "/Game/Input/IMC_Default.IMC_Default" 0 (struct))
  (`EnhancedInputSubsystemInterface.RemoveMappingContext` _returnvalue_2 "/Game/Input/IMC_Tasks.IMC_Tasks" (struct))
  (set `/Game/Features/PaperSorting/BP_SortingDesk.Interacted` false (`/Game/Features/PaperSorting/BP_SortingMinigame.SortingDesk` _sortingminigameref))
  (`/Game/Features/PaperSorting/BP_SortingMinigame.RestartMinigame` _sortingminigameref)
  (`/Game/Players/BP_PlayerController.OnTaskCompletedOnce` _playercontrollerref (`GameplayStatics.GetPlayerControllerID` _playercontrollerref))
  (`/Game/Players/BP_PlayerCharacter.Event MinigameExited` (`/Game/Features/PaperSorting/BP_SortingMinigame.PlayerCharacterRef` (`self.SortingMinigameRef`))))

(fn `ResetCameraRotation`
  (`SceneComponent.K2_SetWorldRotation` (`self.Camera`) (`self.CameraOriginalRotation`) false false))

(fn `SetPlayerPosition`
  (bind _sortingminigameref (`self.SortingMinigameRef`))
  (bind _playerstandlocation (`/Game/Features/PaperSorting/BP_SortingMinigame.PlayerStandLocation` _sortingminigameref))
  (`self.K2_SetActorLocationAndRotation` (`/Game/Features/PaperSorting/BP_SortingMinigame.PlayerCharacterRef` _sortingminigameref) (`SceneComponent.K2_GetComponentLocation` _playerstandlocation) (`SceneComponent.K2_GetComponentRotation` _playerstandlocation) false true))

(fn `UserConstructionScript`)